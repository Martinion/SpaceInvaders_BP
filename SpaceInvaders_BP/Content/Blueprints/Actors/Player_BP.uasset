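; Player actor that moves from input axes and fires bullets on left mouse click.
; Tick moves it on X and Y by axis values scaled by speed and delta time, without sweep.
; Each click spawns a Bullet at the actor's transform, rate-limited by comparing game time to the last shot.
; Overlapping a Game_Over_BP while the X input is positive shifts it by BarrierDisplacement along X to restrict the play area.
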(event EventBeginPlay)

(event Collision|EventActorBeginOverlap
  (params (OtherActor :type Actor%20Object%20Reference))
  ;[1 1 1] Restrict player area
  (Utilities|Casting|CastToGame_Over_BP OtherActor)
  (if (> (Input|AxisValues|GetMoveX) 0.0)
    (Transformation|SetActorLocation (+ (Transformation|GetActorLocation) (Math|Vector|MakeVector (Variables|Default|GetBarrierDisplacement) 0.0 0.0)) false false)))

(event EventTick
  (params (DeltaSeconds :type Float%20%28single-precision%29))
  ;[1 1 1] Movement
  (Transformation|SetActorLocation (+ (Transformation|GetActorLocation) (* (Math|Vector|MakeVector (Input|AxisValues|GetMoveX) (Input|AxisValues|GetMoveY) 0.0) (* DeltaSeconds (Variables|Default|GetMovementSpeed)))) false false))

(event Input|MouseEvents|LeftMouseButton
  (params (Key :type Key%20Structure))
  ;[1 1 1] Shooting
  (:Pressed
    (if (> (Utilities|Time|GetTimeSeconds) (+ (Variables|Default|GetLastBulletFired) (Variables|Default|GetBulletShootingSpeed)))
      (Game|SpawnActorfromClass "/Game/Blueprints/Actors/Bullet.Bullet_C" (Transformation|GetActorTransform) "Undefined" 0 0)
      (Variables|Default|SetLastBulletFired (Utilities|Time|GetTimeSeconds)))))

(fn ConstructionScript)