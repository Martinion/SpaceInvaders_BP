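; Enemy actor Blueprint that advances along negative X in a stepped zigzag, alternating forward moves with sideways shifts.
; Tick moves it without sweep by axis speed and delta time, along either negative X or positive or negative Y.
; A game-time check switches phase at a set interval, using nested FlipFlops to cycle forward, positive Y, forward, negative Y through two direction booleans.
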(event EventBeginPlay)

(event EventTick
  (params (DeltaSeconds :type Float%20%28single-precision%29))
  (bind _movementspeedy (Variables|Default|GetMovementSpeedY))
  (bind _returnvalue (* DeltaSeconds _movementspeedy))
  (if (Variables|Default|GetIfMoveX)
    (Transformation|SetActorLocation (- (Transformation|GetActorLocation) (Math|Vector|MakeVector (* DeltaSeconds (Variables|Default|GetMovementSpeedX)) 0.0 0.0)) false false)
    (elif (Variables|Default|GetIfMovePosY)
      (Transformation|SetActorLocation (+ (Transformation|GetActorLocation) (Math|Vector|MakeVector 0.0 _returnvalue 0.0)) false false)
      (else
        (Transformation|SetActorLocation (- (Transformation|GetActorLocation) (Math|Vector|MakeVector 0.0 _returnvalue 0.0)) false false))))
  (if (> (Utilities|Time|GetTimeSeconds) (Variables|Default|GetLastMoveStart))
    (Variables|Default|SetLastMoveStart (+ (Utilities|Time|GetTimeSeconds) (Variables|Default|GetTimeBetweenMovementChange)))
    (Utilities|FlowControl|FlipFlop
      (:A
        (Variables|Default|SetIfMoveX true))
      (:B
        (Utilities|FlowControl|FlipFlop
          (:A
            (Variables|Default|SetIfMovePosY true)
            (Variables|Default|SetIfMoveX false))
          (:B
            (Variables|Default|SetIfMovePosY false)
            (Variables|Default|SetIfMoveX false)))))))

(fn ConstructionScript)